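; Card actor that plays animations for drawing, summoning servants, casting spells and attacking, and responds to cursor hover.
; Each Start event calls its parent, creates a Level Sequence player that keeps its end state, and binds the card at runtime to an ownership-selected binding.
; Finished callbacks are bound before playback, with one omitted when the card is being attacked.
; Hovering switches card state from Lerp to Focus, and leaving reverts it.
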(event EventStartDrawCard
  (params (Owning :type Boolean) (Package :type Event%20Package%20Struct%20Structure%20%28by%20ref%29))
  (|CallParentFunction Owning Package)
  (bind (_outactor _returnvalue) (Sequencer|Player|CreateLevelSequencePlayer "/Game/LevelSequence/DrawCardSequence.DrawCardSequence" (Utilities|Struct|MakeMovieSceneSequencePlaybackSettings false "(Value=0)" "(TickIntervalSeconds=0.000000,EvaluationBudgetMicroseconds=0.000000,bTickWhenPaused=False,bAllowRounding=True)" 1.0 0.0 false false false false false false "ForceKeepState" false)))
  (Class|LevelSequenceActor|AddBinding _outactor (select Owning (|GetSequenceBinding) (|GetSequenceBinding)) self false)
  (EventDispatchers|BindEventtoOnFinished _returnvalue (EventDispatchers|CreateEvent self :!event EndDrawCard))
  (EventDispatchers|BindEventtoOnFinished _returnvalue (EventDispatchers|CreateEvent _outactor :!event K2DestroyActor))
  (Sequencer|Player|Play _returnvalue :!class /Script/MovieScene.MovieSceneSequencePlayer))

(event EventStartSummonServant
  (params (Owning :type Boolean) (Package :type Event%20Package%20Struct%20Structure%20%28by%20ref%29))
  (|CallParentFunction Owning Package)
  (bind (_outactor _returnvalue) (Sequencer|Player|CreateLevelSequencePlayer "/Game/LevelSequence/SummonServantSequence.SummonServantSequence" (Utilities|Struct|MakeMovieSceneSequencePlaybackSettings false "(Value=0)" "(TickIntervalSeconds=0.000000,EvaluationBudgetMicroseconds=0.000000,bTickWhenPaused=False,bAllowRounding=True)" 1.0 0.0 false false false false false false "ForceKeepState" false)))
  (Class|LevelSequenceActor|AddBinding _outactor (select Owning (|GetSequenceBinding) (|GetSequenceBinding)) self false)
  (EventDispatchers|BindEventtoOnFinished _returnvalue (EventDispatchers|CreateEvent self :!event EndSummonServant))
  (EventDispatchers|BindEventtoOnFinished _returnvalue (EventDispatchers|CreateEvent _outactor :!event K2DestroyActor))
  (Sequencer|Player|Play _returnvalue :!class /Script/MovieScene.MovieSceneSequencePlayer))

(event EventStartCastSpell
  (params (Owning :type Boolean) (Package :type Event%20Package%20Struct%20Structure%20%28by%20ref%29))
  (|CallParentFunction Owning Package)
  (bind (_outactor _returnvalue) (Sequencer|Player|CreateLevelSequencePlayer "/Game/LevelSequence/CastSpellSequence.CastSpellSequence" (Utilities|Struct|MakeMovieSceneSequencePlaybackSettings false "(Value=0)" "(TickIntervalSeconds=0.000000,EvaluationBudgetMicroseconds=0.000000,bTickWhenPaused=False,bAllowRounding=True)" 1.0 0.0 false false false false false false "ForceKeepState" false)))
  (Class|LevelSequenceActor|AddBinding _outactor (select Owning (|GetSequenceBinding) (|GetSequenceBinding)) self false)
  (EventDispatchers|BindEventtoOnFinished _returnvalue (EventDispatchers|CreateEvent self :!event EndCastSpell))
  (EventDispatchers|BindEventtoOnFinished _returnvalue (EventDispatchers|CreateEvent _outactor :!event K2DestroyActor))
  (Sequencer|Player|Play _returnvalue :!class /Script/MovieScene.MovieSceneSequencePlayer))

(event EventStartAttack
  (params (BeAttacked :type Boolean) (Owning :type Boolean) (Package :type Event%20Package%20Struct%20Structure%20%28by%20ref%29))
  (|CallParentFunction BeAttacked Owning Package)
  (bind (_outactor _returnvalue) (Sequencer|Player|CreateLevelSequencePlayer "/Game/LevelSequence/AttackAndAttackedSequence.AttackAndAttackedSequence" (Utilities|Struct|MakeMovieSceneSequencePlaybackSettings false "(Value=0)" "(TickIntervalSeconds=0.000000,EvaluationBudgetMicroseconds=0.000000,bTickWhenPaused=False,bAllowRounding=True)" 1.0 0.0 false false false false false false "ForceKeepState" false)))
  (Class|LevelSequenceActor|AddBinding _outactor (select Owning (|GetSequenceBinding) (|GetSequenceBinding)) self false)
  (if (not BeAttacked)
    (EventDispatchers|BindEventtoOnFinished _returnvalue (EventDispatchers|CreateEvent self :!event EndAttack)))
  (EventDispatchers|BindEventtoOnFinished _returnvalue (EventDispatchers|CreateEvent _outactor :!event K2DestroyActor))
  (Sequencer|Player|Play _returnvalue :!class /Script/MovieScene.MovieSceneSequencePlayer))

(event OnBeginCursorOver(CardCollision)
  (params (TouchedComponent :type Primitive%20Component%20Object%20Reference))
  (switch Utilities|FlowControl|Switch|SwitchonEState (Variables|Default|GetCardState)
    (:Lerp
      (Class|CardModel|SetCardState "Focus"))))

(event OnEndCursorOver(CardCollision)
  (params (TouchedComponent :type Primitive%20Component%20Object%20Reference))
  (switch Utilities|FlowControl|Switch|SwitchonEState (Variables|Default|GetCardState)
    (:Focus
      (Class|CardModel|SetCardState "Lerp"))))

(fn ConstructionScript)